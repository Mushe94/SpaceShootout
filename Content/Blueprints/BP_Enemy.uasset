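; Robot enemy for an FPS that awards the player points when a bullet kills it.
; BeginPlay caches the player and robot AnimInstance, and Tick copies the player's alive state and feeds IsMoving to the animation's PlayerFound flag.
; Separate Head and Body overlaps award their own score if EnemyLife is depleted, then spawn effects and destroy the actor.
; EnemyLife and IsMoving are only read in these graphs, never set.
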(event OnComponentBeginOverlap(Body)
  (params (OverlappedComponent :type Primitive%20Component%20Object%20Reference) (OtherActor :type Actor%20Object%20Reference) (OtherComp :type Primitive%20Component%20Object%20Reference) (OtherBodyIndex :type Integer) (bFromSweep :type Boolean) (SweepResult :type Hit%20Result%20Structure%20%28by%20ref%29))
  (bind _returnvalue (Transformation|GetActorLocation))
  (Utilities|Casting|CastToBullet OtherActor)
  (if (<= (Variables|Default|GetenemyLife) 0.0)
    (Class|FPSController|UpdatePoints (Variables|Default|GetPlayer) (Variables|Default|GetbodyScore))
    (Effects|SpawnEmitteratLocation "/Game/TS_Fireworks/Particles/PS_TS_Fireworks_Burst_Circle.PS_TS_Fireworks_Burst_Circle" _returnvalue)
    (Audio|PlaySoundatLocation "/Game/Blueprints/Audio/RobotDeath.RobotDeath" _returnvalue "0, 0, 0" 1.0 1.0 0.0 0 0 0)
    (Actor|DestroyActor)))

(event OnComponentBeginOverlap(Head)
  (params (OverlappedComponent :type Primitive%20Component%20Object%20Reference) (OtherActor :type Actor%20Object%20Reference) (OtherComp :type Primitive%20Component%20Object%20Reference) (OtherBodyIndex :type Integer) (bFromSweep :type Boolean) (SweepResult :type Hit%20Result%20Structure%20%28by%20ref%29))
  (bind _returnvalue (Transformation|GetActorLocation))
  (Utilities|Casting|CastToBullet OtherActor)
  (if (<= (Variables|Default|GetenemyLife) 0.0)
    (Class|FPSController|UpdatePoints (Variables|Default|GetPlayer) (Variables|Default|GetheadScore))
    (Effects|SpawnEmitteratLocation "/Game/TS_Fireworks/Particles/PS_TS_Fireworks_Burst_Circle.PS_TS_Fireworks_Burst_Circle" _returnvalue)
    (Audio|PlaySoundatLocation "/Game/Blueprints/Audio/RobotDeath.RobotDeath" _returnvalue "0, 0, 0" 1.0 1.0 0.0 0 0 0)
    (Actor|DestroyActor)))

(event EventBeginPlay
  (bind _asbp_fpscontroller (Utilities|Casting|CastToBP_FPSController (Game|GetPlayerCharacter 0)))
  (Variables|Default|SetPlayer _asbp_fpscontroller)
  (bind _asbp_robot_animations (Utilities|Casting|CastToBP_RobotAnimations (Components|SkeletalMesh|GetAnimInstance (Variables|Default|GetSkeletalMesh))))
  (Variables|Default|SetAnim _asbp_robot_animations))

(event EventTick
  (params (DeltaSeconds :type Float%20%28single-precision%29))
  (Variables|Default|SetisPlayerAlive (Variables|/Script/SpaceShootout.FPSController|GetisAlive (Variables|Default|GetPlayer)))
  (Variables|/Game/Blueprints/Animations/BP_RobotAnimations.BP_RobotAnimations_C|SetPlayerFound (Variables|Default|GetAnim) (Variables|Default|GetisMoving)))

(fn ConstructionScript)