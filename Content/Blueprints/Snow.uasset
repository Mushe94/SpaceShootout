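; Snow zone actor that slows the BP_FPSController player while overlapped and drives an ice effect through a material parameter collection.
; Begin overlap applies the slow movement speed and sets an active flag; end overlap restores the player cached at BeginPlay, without checking which actor left.
; Tick ramps the IceAmount scalar in SnowCollection up while active and down otherwise, clamped between zero and one.
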(event EventBeginPlay
  (bind _returnvalue (Actor|GetActorOfClass "/Game/Blueprints/BP_FPSController.BP_FPSController_C"))
  (Variables|Default|Setplayer _returnvalue))

(event Collision|EventActorBeginOverlap
  (params (OtherActor :type Actor%20Object%20Reference))
  (bind _asbp_fpscontroller (Utilities|Casting|CastToBP_FPSController OtherActor))
  (Class|FPSController|ModifyMovementSpeed _asbp_fpscontroller (Variables|Default|GetslowMovementSpeed))
  (Variables|Default|SetisActive true))

(event EventTick
  (params (DeltaSeconds :type Float%20%28single-precision%29))
  (if (Variables|Default|GetisActive)
    (bind _returnvalue (Rendering|Material|GetScalarParameterValue "/Game/Blueprints/SnowCollection.SnowCollection" "IceAmount" :!class /Script/Engine.KismetMaterialLibrary))
    (Rendering|Material|SetScalarParameterValue "/Game/Blueprints/SnowCollection.SnowCollection" "IceAmount" (Math|Float|Clamp(Float) (+ _returnvalue DeltaSeconds)) :!class /Script/Engine.KismetMaterialLibrary)
    (else
      (bind _returnvalue_2 (Rendering|Material|GetScalarParameterValue "/Game/Blueprints/SnowCollection.SnowCollection" "IceAmount" :!class /Script/Engine.KismetMaterialLibrary))
      (Rendering|Material|SetScalarParameterValue "/Game/Blueprints/SnowCollection.SnowCollection" "IceAmount" (Math|Float|Clamp(Float) (- _returnvalue_2 DeltaSeconds)) :!class /Script/Engine.KismetMaterialLibrary))))

(event Collision|EventActorEndOverlap
  (params (OtherActor :type Actor%20Object%20Reference))
  (Class|FPSController|RestoreMovementSpeed (Variables|Default|Getplayer))
  (Variables|Default|SetisActive false))

(fn ConstructionScript)