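; BP_Bullet is a projectile that damages the FPSController or Enemy actors it hits, ignoring the one stored as MyOwner.
; Its Box overlap casts the other actor to each type, skips immortal FPSControllers, then applies damage, plays type-specific and impact sounds, and destroys itself.
; Other actors trigger only the impact sound, with the bullet destroyed only if that actor is its GetOwner result.
; BeginPlay assigns the Bullet component to BulletStaticMesh.
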(event OnComponentBeginOverlap(Box)
  (params (OverlappedComponent :type Primitive%20Component%20Object%20Reference) (OtherActor :type Actor%20Object%20Reference) (OtherComp :type Primitive%20Component%20Object%20Reference) (OtherBodyIndex :type Integer) (bFromSweep :type Boolean) (SweepResult :type Hit%20Result%20Structure%20%28by%20ref%29))
  (bind _returnvalue (Transformation|GetActorLocation))
  (bind _damage (Variables|Default|Getdamage))
  (bind _myowner (Variables|Default|GetmyOwner))
  (bind _asfpscontroller (Utilities|Casting|CastToFPSController OtherActor)
    (:then
      (if (not (== _myowner _asfpscontroller))
        (if (not (Variables|/Script/SpaceShootout.FPSController|GetisImmortal _asfpscontroller))
          (Class|FPSController|TakeDamage _asfpscontroller _damage)
          (Audio|PlaySoundatLocation "/Game/Blueprints/Audio/Human-Grunt.Human-Grunt" (Transformation|GetActorLocation _asfpscontroller) "0, 0, 0" 1.0 1.0 0.0 0 0 0)
          (Audio|PlaySoundatLocation "/Game/Blueprints/Audio/BulletImpact.BulletImpact" _returnvalue "0, 0, 0" 1.0 1.0 0.0 0 0 0)
          (Actor|DestroyActor))))
    (:CastFailed
      (bind _asenemy (Utilities|Casting|CastToEnemy OtherActor)
        (:then
          (if (not (== _myowner _asenemy))
            (Class|Enemy|TakeDamage _asenemy _damage)
            (Audio|PlaySoundatLocation "/Game/Blueprints/Audio/RobotImpact.RobotImpact" (Transformation|GetActorLocation _asenemy) "0, 0, 0" 1.0 1.0 0.0 0 0 0)
            (Audio|PlaySoundatLocation "/Game/Blueprints/Audio/BulletImpact.BulletImpact" _returnvalue "0, 0, 0" 1.0 1.0 0.0 0 0 0)
            (Actor|DestroyActor)))
        (:CastFailed
          (Audio|PlaySoundatLocation "/Game/Blueprints/Audio/BulletImpact.BulletImpact" _returnvalue "0, 0, 0" 1.0 1.0 0.0 0 0 0)
          (if (== OtherActor (Components|GetOwner))
            (Actor|DestroyActor)))))))

(event EventBeginPlay
  (Variables|Default|SetbulletStaticMesh (Variables|Default|GetBullet)))

(fn ConstructionScript)