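; BP_FPSController is a first-person Blueprint that manages the HUD and the death-to-respawn cycle.
; On BeginPlay it creates the UI widget and adds it to the viewport.
; Tick polls CurrentLife and clears IsAlive once it drops to zero or below.
; While IsAlive is false, Tick runs a five-second Delay and then calls Respawn, which is not defined in these graphs.
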(event EventBeginPlay
  (bind _returnvalue (UserInterface|CreateWidget "/Game/Blueprints/UI.UI_C"))
  (bind _output_get (Variables|Default|SetUI _returnvalue))
  (UserInterface|Viewport|AddtoViewport _output_get 0))

(event Collision|EventActorBeginOverlap
  (params (OtherActor :type Actor%20Object%20Reference)))

(event EventTick
  (params (DeltaSeconds :type Float%20%28single-precision%29))
  (if (Variables|Default|GetisAlive)
    (if (<= (Variables|Default|GetcurrentLife) 0.0)
      (Variables|Default|SetisAlive false))
    (else
      (Utilities|FlowControl|Delay 5.0)
      (Class|FPSController|Respawn))))

(fn ConstructionScript)